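; Bottle actor that disables gravity on the player pawn's mesh for a few seconds when the player enters its sphere.
; Sphere overlaps with the player toggle a CanInteract flag and a widget, hidden at BeginPlay.
; The gravity effect fires directly on overlap via a DefaultPawn_BP cast, and a Delay restores gravity regardless of exit.
; CanInteract is set but never read in this graph.
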(event OnComponentBeginOverlap(Sphere)
  (params (OverlappedComponent :type Primitive%20Component%20Object%20Reference) (OtherActor :type Actor%20Object%20Reference) (OtherComp :type Primitive%20Component%20Object%20Reference) (OtherBodyIndex :type Integer) (bFromSweep :type Boolean) (SweepResult :type Hit%20Result%20Structure%20%28by%20ref%29))
  (if (== OtherActor (Game|Player|GetPlayerPawn 0))
    (Variables|Default|SetCanInteract true)
    (Rendering|SetVisibility (Variables|Default|GetWidget) true false)
    (bind _asdefault_pawn_bp (Utilities|Casting|CastToDefaultPawn_BP (Game|Player|GetPlayerPawn 0)))
    (Physics|SetEnableGravity (Variables|/Script/Engine.DefaultPawn|GetMeshComponent _asdefault_pawn_bp) false)
    (Utilities|FlowControl|Delay 5.0)
    (bind _asdefault_pawn_bp_2 (Utilities|Casting|CastToDefaultPawn_BP (Game|Player|GetPlayerPawn 0)))
    (Physics|SetEnableGravity (Variables|/Script/Engine.DefaultPawn|GetMeshComponent _asdefault_pawn_bp_2) true)))

(event OnComponentEndOverlap(Sphere)
  (params (OverlappedComponent :type Primitive%20Component%20Object%20Reference) (OtherActor :type Actor%20Object%20Reference) (OtherComp :type Primitive%20Component%20Object%20Reference) (OtherBodyIndex :type Integer))
  (if (== (Game|Player|GetPlayerPawn 0) OtherActor)
    (Variables|Default|SetCanInteract false)
    (Rendering|SetVisibility (Variables|Default|GetWidget) false false)))

(event EventBeginPlay
  (Rendering|SetVisibility (Variables|Default|GetWidget) false false))

(fn ConstructionScript)